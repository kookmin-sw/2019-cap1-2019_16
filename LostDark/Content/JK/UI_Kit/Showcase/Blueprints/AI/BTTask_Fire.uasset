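; Behavior tree task in the UI Kit showcase that makes an Example_Enemy fire a bullet at its blackboard target.
; It solves a ballistic toss velocity from the pawn's ProjectileSpawn to the enemy actor's location at a fixed launch speed, tracing only while ascending.
; A valid solution spawns the Bullet with that starting velocity and succeeds; a missing solution or wrong pawn type fails the task.
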(event `self.ReceiveExecute`
  (params (OwnerActor :type "Actor Object Reference"))
  (bind _returnvalue (`AIBlueprintHelperLibrary.GetAIController` OwnerActor))
  (bind _asexample_enemy (cast `/Game/UI_Kit/Showcase/Blueprints/Example_Enemy` (`Controller.K2_GetPawn` _returnvalue))
    (:`then`
      (bind _returnvalue_2 (`SceneComponent.K2_GetComponentLocation` (`/Game/UI_Kit/Showcase/Blueprints/Example_Enemy.Projectile Spawn` _asexample_enemy)))
      (bind (_tossvelocity _returnvalue_3) (`GameplayStatics.BlueprintSuggestProjectileVelocity` _returnvalue_2 (`Actor.K2_GetActorLocation` (cast `Actor` (`BlackboardComponent.GetValueAsObject` (`AIBlueprintHelperLibrary.GetBlackboard` _returnvalue) (`self.BBKey_Enemy`)) :!pure true)) 3000.0 0.0 "OnlyTraceWhileAscending" 30.0))
      (if _returnvalue_3
        (`|SpawnActorFromClass` "/Game/UI_Kit/Showcase/Blueprints/Bullet.Bullet_C" (`KismetMathLibrary.Conv_VectorToTransform` _returnvalue_2) "Undefined" "OverrideRootScale" null _tossvelocity)
        (`self.FinishExecute` true)
        (else
          (`self.FinishExecute` false))))
    (:`CastFailed`
      (`self.FinishExecute` false))))