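; BP_CharacterPawn is the Lava Knight character pawn, handling basic player look and movement input.
; LookUp and Turn axes feed controller pitch and yaw input directly.
; MoveForward and MoveRight rotate forward and right vectors by the control rotation's yaw only, so movement follows the camera heading while staying horizontal.
; The construction script is empty.
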(event `InputAxis|LookUp` :overrideparent false
  (params (AxisValue :type "Float (single-precision)"))
  (`self.AddControllerPitchInput` AxisValue))

(event `InputAxis|Turn` :overrideparent false
  (params (AxisValue :type "Float (single-precision)"))
  (`self.AddControllerYawInput` AxisValue))

(event `InputAxis|MoveForward` :overrideparent false
  (params (AxisValue :type "Float (single-precision)"))
  (`self.AddMovementInput` (`KismetMathLibrary.GreaterGreater_VectorRotator` (1.0 0.0 0.0) (`KismetMathLibrary.MakeRot` 0.0 (.yaw (`Controller.GetControlRotation` (`self.GetController`))))) AxisValue))

(event `InputAxis|MoveRight` :overrideparent false
  (params (AxisValue :type "Float (single-precision)"))
  (`self.AddMovementInput` (`KismetMathLibrary.GreaterGreater_VectorRotator` (0.0 1.0 0.0) (`KismetMathLibrary.MakeRot` 0.0 (.yaw (`Controller.GetControlRotation` (`self.GetController`))))) AxisValue))

(fn `UserConstructionScript`)