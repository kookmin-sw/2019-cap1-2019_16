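; Bear mob Blueprint that defines the bear's melee attack damage.
; When the attack begins, it sphere-traces a short distance forward against one object type and applies fixed point damage to the hit actor, with its controller as instigator.
; The trace still draws timed debug shapes; attack end is empty, and BeginPlay, Tick and overlap are disabled stubs.
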(event `OnAttackBegin`
  (bind _returnvalue (`self.K2_GetActorLocation`))
  ;[1 1 1] 영역에 따라 데미지를 입힘
  (bind (_outhit _returnvalue_2) (`KismetSystemLibrary.SphereTraceSingleForObjects` :`Start` _returnvalue :`End` (+ (* (`self.GetActorForwardVector`) 200.0) _returnvalue) :`Radius` 100.0 :`ObjectTypes` (`|MakeArray` "ObjectTypeQuery7" :!type "EObjectTypeQuery Enum") :`DrawDebugType` "ForDuration"))
  (if _returnvalue_2
    (`GameplayStatics.ApplyPointDamage` (`.HitActor` (`GameplayStatics.BreakHitResult` _outhit)) 50.0 (`self.GetActorForwardVector`) _outhit (`self.GetController`))))

(event `OnAttackEnd`
  ;[1 1 1] 영역에 따라 데미지를 입힘
)

(fn `UserConstructionScript`
  (`parent.UserConstructionScript`))