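; Ranged Frost Giant mob Blueprint, stored in a NotUse folder, that adjusts its walk speed by AI state.
; Tick calls the parent, then sets the movement component's max walk speed from the current pawn state, with Peace and Chase using the same speed.
; BeginPlay is empty with its parent call disconnected, the overlap event is disabled, and the construction script only calls the parent.
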(event `self.ReceiveBeginPlay`)

(event `self.ReceiveTick`
  (params (DeltaSeconds :type "Float (single-precision)"))
  (`parent.ReceiveTick` DeltaSeconds)
  (switch `/Game/YR/Mobs/BPE_EnemyState` (`self.CurrentStatePawn`) ; 현재 State에 따라 다른 속도 값
    (:`NewEnumerator0`
      (set `CharacterMovementComponent.MaxWalkSpeed` 100.0 (`self.CharacterMovement`)))
    (:`NewEnumerator1`
      (set `CharacterMovementComponent.MaxWalkSpeed` 100.0 (`self.CharacterMovement`)))))

(fn `UserConstructionScript`
  (`parent.UserConstructionScript`))