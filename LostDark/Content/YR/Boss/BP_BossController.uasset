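; BP_BossController is the boss's AI controller, deciding how it moves in its peace state.
; On possess it first initializes the BP_BossBB blackboard, storing the pawn's spawn location as home, an idle time, and a random navigable point within a radius as the first target.
; It then starts the BP_BossBT behavior tree, which uses those blackboard values.
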(event `self.OnPossess`
  (params (PossessedPawn :type "Pawn Object Reference"))
  (bind _returnvalue (`self.K2_GetActorLocation` (`self.K2_GetPawn`)))
  ;[1 1 1] Enemy Controller - PEACE 상태에서 Enemy가 움직이는 방식을 결정
  (`|ExecutionSequence`
    (:`then_0`
      (`self.UseBlackboard` "/Game/YR/Boss/BP_BossBB.BP_BossBB") ; 먼저 블랙보드 사용
      (`BlackboardComponent.SetValueAsVector` (`self.Blackboard`) (`self.HomeLocationKey`) _returnvalue) ; Get Blackboard 한 뒤 벡터값 초기화
      (`BlackboardComponent.SetValueAsFloat` (`self.Blackboard`) (`self.IdleTimeKey`) 4.0)
      (`BlackboardComponent.SetValueAsVector` (`self.Blackboard`) (`self.TargetLocationKey`) (`NavigationSystemV1.K2_GetRandomLocationInNavigableRadius` _returnvalue (`self.NewLocationRadius`) null null)))
    (:`then_1`
      (`self.RunBehaviorTree` "/Game/YR/Boss/BP_BossBT.BP_BossBT") ; 그 다음 Behavior Tree 사용
    )))

(fn `UserConstructionScript`)