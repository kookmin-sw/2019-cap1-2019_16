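; Griffon boss Blueprint that executes a basic attack and three telegraphed skills: fire/dark storm, lightning and ice laser.
; Warning events briefly reveal indicators, while Begin events time particles and screech sounds with delays, then destroy the emitters.
; Each attack uses a single-hit sphere trace with debug drawing to apply point damage, skipped in one CurrentStatePawn state.
; All three skill Begins hide Warning3; End events are empty.
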(event `SKILL2Begin`
  (bind _returnvalue (`SceneComponent.GetSocketLocation` (`self.skill2Loc`) "None"))
  ;[1 1 1] SKILL2
  (`KismetSystemLibrary.Delay` 0.4)
  (bind _returnvalue_2 (`GameplayStatics.SpawnEmitterAtLocation` "/Game/FXVarietyPack/Particles/P_ky_healAura.P_ky_healAura" (`self.K2_GetActorLocation`) (struct) (6.0 6.0 6.0)))
  (`KismetSystemLibrary.Delay` 0.1)
  (bind _returnvalue_3 (`GameplayStatics.SpawnEmitterAtLocation` "/Game/FXVarietyPack/Particles/P_ky_ThunderBallHit.P_ky_ThunderBallHit" _returnvalue (struct) (5.0 6.0 5.0)))
  (bind _returnvalue_4 (`GameplayStatics.SpawnEmitterAtLocation` "/Game/FXVarietyPack/Particles/P_ky_lightning3.P_ky_lightning3" _returnvalue (struct) (3.0 3.0 3.0)))
  (bind _returnvalue_5 (`GameplayStatics.SpawnEmitterAtLocation` "/Game/FXVarietyPack/Particles/P_ky_thunderBall.P_ky_thunderBall" (`SceneComponent.GetSocketLocation` (`self.skill2startpoint`) "None") (struct) (5.0 6.0 5.0)))
  (bind _returnvalue_6 (`GameplayStatics.SpawnEmitterAtLocation` "/Game/FXVarietyPack/Particles/P_ky_thunderBall.P_ky_thunderBall" (`SceneComponent.GetSocketLocation` (`self.skill2endpoint`) "None") (struct) (5.0 6.0 5.0)))
  (`GameplayStatics.SpawnSoundAttached` "/Game/YR/효과음/hawk_screeching-Mike_Koenig-1626170357.hawk_screeching-Mike_Koenig-1626170357" (`self.Capsule`) "None" (`self.K2_GetActorLocation`) (struct) "KeepRelativeOffset" false 1.0 1.0 0.0 null null)
  (bind (_outhit _returnvalue_7) (`KismetSystemLibrary.SphereTraceSingleForObjects` :`Start` (`SceneComponent.GetSocketLocation` (`self.skill2startpoint`) "None") :`End` (`SceneComponent.GetSocketLocation` (`self.skill2endpoint`) "None") :`Radius` 500.0 :`ObjectTypes` (`|MakeArray` "ObjectTypeQuery7" :!type "EObjectTypeQuery Enum") :`DrawDebugType` "ForDuration"))
  (`SceneComponent.SetHiddenInGame` (`self.Warning3`) true false)
  (if _returnvalue_7
    (if (`|EnumInequality` (`self.CurrentStatePawn`) "NewEnumerator3")
      (`GameplayStatics.ApplyPointDamage` (`.HitActor` (`GameplayStatics.BreakHitResult` _outhit)) 3.0 (`self.GetActorForwardVector`) _outhit (`self.GetController`))))
  (`KismetSystemLibrary.Delay` 1.0)
  (`ActorComponent.K2_DestroyComponent` _returnvalue_2)
  (`ActorComponent.K2_DestroyComponent` _returnvalue_3)
  (`ActorComponent.K2_DestroyComponent` _returnvalue_5)
  (`ActorComponent.K2_DestroyComponent` _returnvalue_6)
  (`ActorComponent.K2_DestroyComponent` _returnvalue_4))

(event `SKILL2End`
  ;[1 1 1] SKILL2
)

(event `OnAttackBeginBoss`
  ;[1 1 1] 영역에 따라 데미지를 입힘
  (bind (_outhit _returnvalue) (`KismetSystemLibrary.SphereTraceSingleForObjects` :`Start` (+ (`self.K2_GetActorLocation`) (0.0 0.0 -100.0)) :`End` (`SceneComponent.GetSocketLocation` (`self.AttackLoc`) "None") :`Radius` 130.0 :`ObjectTypes` (`|MakeArray` "ObjectTypeQuery7" :!type "EObjectTypeQuery Enum") :`DrawDebugType` "ForDuration"))
  (`GameplayStatics.SpawnEmitterAttached` "/Game/FXVarietyPack/Particles/P_ky_shotShockwave.P_ky_shotShockwave" (`self.attackEffec`) "None" (0.0 0.0 0.0) (struct) (2.0 2.0 2.0))
  (if _returnvalue
    (if (`|EnumInequality` (`self.CurrentStatePawn`) "NewEnumerator3")
      (`GameplayStatics.ApplyPointDamage` (`.HitActor` (`GameplayStatics.BreakHitResult` _outhit)) 50.0 (`self.GetActorForwardVector`) _outhit (`self.GetController`)))))

(event `SKILL2Warning`
  (bind _warning2 (`self.Warning2`))
  ;[1 1 1] SKILL2
  (`SceneComponent.SetHiddenInGame` _warning2 false false)
  (`KismetSystemLibrary.Delay` 2.0)
  (`SceneComponent.SetHiddenInGame` _warning2 true false))

(event `OnAttackEndBoss`
  ;[1 1 1] 영역에 따라 데미지를 입힘
)

(event `SKILL3Begin`
  (bind _floorplane (`self.FloorPlane`))
  (bind _mouse (`self.Mouse`))
  ;[1 1 1] SKILL3
  (`KismetSystemLibrary.Delay` 0.4)
  (bind _returnvalue (`GameplayStatics.SpawnEmitterAttached` "/Game/FXVarietyPack/Particles/P_ky_waterBall.P_ky_waterBall" _mouse "None" (0.0 0.0 0.0) (struct) (2.0 2.0 2.0)))
  (bind _returnvalue_2 (`GameplayStatics.SpawnEmitterAttached` "/Game/FXVarietyPack/Particles/P_ky_laser01.P_ky_laser01" _mouse "None" (0.0 0.0 0.0) (struct) (2.0 2.0 1.0) "SnapToTarget"))
  (bind _returnvalue_3 (`GameplayStatics.SpawnEmitterAttached` "/Game/FXVarietyPack/Particles/P_ky_laser01.P_ky_laser01" (`self.mouse2`) "None" (0.0 0.0 0.0) (struct) (2.0 2.0 1.0)))
  (bind _returnvalue_4 (`GameplayStatics.SpawnEmitterAttached` "/Game/FXVarietyPack/Particles/P_ky_laser01.P_ky_laser01" (`self.mouse3`) "None" (0.0 0.0 0.0) (struct) (2.0 2.0 1.0)))
  (bind _returnvalue_5 (`GameplayStatics.SpawnEmitterAttached` "/Game/Elemental/Characters/IceKnight/FX/P_FrostGiant_EyeFlare.P_FrostGiant_EyeFlare" _mouse "None" (0.0 0.0 0.0) (struct) (0.5 0.5 0.5)))
  (`KismetSystemLibrary.Delay` 0.1)
  (bind _returnvalue_6 (`GameplayStatics.SpawnEmitterAttached` "/Game/FXVarietyPack/Particles/P_ky_waterBallHit.P_ky_waterBallHit" _floorplane "None" (0.0 0.0 0.0) (struct) (4.0 4.0 4.0) "SnapToTarget"))
  (bind _returnvalue_7 (`GameplayStatics.SpawnEmitterAttached` "/Game/Elemental/Logo/FrozenLogo/_FX_LogoReveal_ICE._FX_LogoReveal_ICE" _floorplane "None" (0.0 0.0 0.0) (struct) (3.0 3.0 3.0) "SnapToTarget"))
  (bind _returnvalue_8 (`GameplayStatics.SpawnEmitterAttached` "/Game/Elemental/Characters/IceKnight/FX/P_FrostGiant_ChestFlare.P_FrostGiant_ChestFlare" _floorplane "None" (0.0 0.0 0.0) (struct) (2.0 2.0 2.0)))
  (`GameplayStatics.SpawnSoundAttached` "/Game/YR/효과음/hawk_screeching-Mike_Koenig-1626170357.hawk_screeching-Mike_Koenig-1626170357" (`self.Capsule`) "None" (`self.K2_GetActorLocation`) (struct) "KeepRelativeOffset" false 1.0 1.0 0.0 null null)
  (bind (_outhit _returnvalue_9) (`KismetSystemLibrary.SphereTraceSingleForObjects` :`Start` (- (`self.K2_GetActorLocation`) (0.0 0.0 50.0)) :`End` (- (`SceneComponent.GetSocketLocation` (`self.FloorPlane`) "None") (0.0 40.0 0.0)) :`Radius` 200.0 :`ObjectTypes` (`|MakeArray` "ObjectTypeQuery7" :!type "EObjectTypeQuery Enum") :`DrawDebugType` "ForDuration"))
  (`SceneComponent.SetHiddenInGame` (`self.Warning3`) true false)
  (if _returnvalue_9
    (if (`|EnumInequality` (`self.CurrentStatePawn`) "NewEnumerator3")
      (`GameplayStatics.ApplyPointDamage` (`.HitActor` (`GameplayStatics.BreakHitResult` _outhit)) 100.0 (`self.GetActorForwardVector`) _outhit (`self.GetController`))))
  (`KismetSystemLibrary.Delay` 0.5)
  (`ActorComponent.K2_DestroyComponent` _returnvalue_2)
  (`ActorComponent.K2_DestroyComponent` _returnvalue)
  (`ActorComponent.K2_DestroyComponent` _returnvalue_7)
  (`ActorComponent.K2_DestroyComponent` _returnvalue_8)
  (`ActorComponent.K2_DestroyComponent` _returnvalue_6)
  (`ActorComponent.K2_DestroyComponent` _returnvalue_5)
  (`ActorComponent.K2_DestroyComponent` _returnvalue_3)
  (`ActorComponent.K2_DestroyComponent` _returnvalue_4))

(event `SKILL3End`
  ;[1 1 1] SKILL3
)

(event `SKILL1Begin`
  (bind _returnvalue (`self.K2_GetActorLocation`))
  (bind _magiccircle (`self.MagicCircle`))
  ;[1 1 1] SKILL1
  (`KismetSystemLibrary.Delay` 1.0)
  (`ActorComponent.K2_DestroyComponent` (stale `SKILL1Warning` _returnvalue))
  (bind _returnvalue_2 (`GameplayStatics.SpawnEmitterAtLocation` "/Game/Elemental/Effects/Fx_Magic/Effects/FX_Knight_Hammer_Powerup.FX_Knight_Hammer_Powerup" _returnvalue))
  (`KismetSystemLibrary.Delay` 0.1)
  (bind _returnvalue_3 (`GameplayStatics.SpawnEmitterAttached` "/Game/FXVarietyPack/Particles/P_ky_explosion.P_ky_explosion" _magiccircle "None" (0.0 0.0 0.0) (struct) (3.0 3.0 3.0) "SnapToTarget"))
  (bind _returnvalue_4 (`GameplayStatics.SpawnEmitterAttached` "/Game/Elemental/Effects/Fx_Magic/Effects/FX_Knight_Torso_Flareup.FX_Knight_Torso_Flareup" _magiccircle))
  (bind _returnvalue_5 (`GameplayStatics.SpawnEmitterAttached` "/Game/FXVarietyPack/Particles/P_ky_fireStorm.P_ky_fireStorm" _magiccircle "None" (0.0 0.0 0.0) (struct) (0.55 0.55 0.55)))
  (bind _returnvalue_6 (`GameplayStatics.SpawnEmitterAttached` "/Game/FXVarietyPack/Particles/P_ky_darkStorm.P_ky_darkStorm" _magiccircle "None" (0.0 0.0 0.0) (struct) (0.4 0.4 0.4)))
  (`GameplayStatics.SpawnSoundAttached` "/Game/YR/효과음/hawk_screeching-Mike_Koenig-1626170357.hawk_screeching-Mike_Koenig-1626170357" (`self.Capsule`) "None" (`self.K2_GetActorLocation`) (struct) "KeepRelativeOffset" false 1.0 1.0 0.0 null null)
  (bind (_outhit _returnvalue_7) (`KismetSystemLibrary.SphereTraceSingleForObjects` :`Start` _returnvalue :`End` _returnvalue :`Radius` 860.0 :`ObjectTypes` (`|MakeArray` "ObjectTypeQuery7" :!type "EObjectTypeQuery Enum") :`DrawDebugType` "ForDuration"))
  (`SceneComponent.SetHiddenInGame` (`self.Warning3`) true false)
  (if _returnvalue_7
    (if (`|EnumInequality` (`self.CurrentStatePawn`) "NewEnumerator3")
      (`GameplayStatics.ApplyPointDamage` (`.HitActor` (`GameplayStatics.BreakHitResult` _outhit)) 150.0 (`self.GetActorForwardVector`) _outhit (`self.GetController`))))
  (`KismetSystemLibrary.Delay` 1.0)
  (`ActorComponent.K2_DestroyComponent` _returnvalue_2)
  (`ActorComponent.K2_DestroyComponent` _returnvalue_3)
  (`ActorComponent.K2_DestroyComponent` _returnvalue_4)
  (`ActorComponent.K2_DestroyComponent` _returnvalue_5)
  (`ActorComponent.K2_DestroyComponent` _returnvalue_6))

(event `SKILL1End`
  ;[1 1 1] SKILL1
)

(event `SKILL3Warning`
  ;[1 1 1] SKILL3
  (`SceneComponent.SetHiddenInGame` (`self.Warning3`) false false)
  (`KismetSystemLibrary.Delay` 2.0)
  (`SceneComponent.SetHiddenInGame` (`self.Warning3`) true false))

(event `SKILL1Warning`
  ;[1 1 1] SKILL1
  (`SceneComponent.SetHiddenInGame` (`self.Warning1`) false false)
  (bind _returnvalue (`GameplayStatics.SpawnEmitterAttached` "/Game/FXVarietyPack/Particles/P_ky_magicCircle1.P_ky_magicCircle1" (`self.MagicCircle`) "None" (0.0 0.0 0.0) (struct) (0.7 0.7 0.7)))
  (`KismetSystemLibrary.Delay` 1.5)
  (`SceneComponent.SetHiddenInGame` (`self.Warning1`) true false))

(fn `UserConstructionScript`
  (`parent.UserConstructionScript`))