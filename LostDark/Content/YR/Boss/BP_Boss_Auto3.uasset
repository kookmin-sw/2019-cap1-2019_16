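; BP_Boss_Auto3 is a boss pawn with a state machine (peace, chase, attack, three skills, dead) mirrored to its AI Blackboard.
; Sighting a pawn during peace starts a chase, which randomizes walk speed and writes a random attack choice to the Blackboard.
; Damage reveals the health bar and reduces HP until the boss locks into the dead state, while Tick updates the bar.
; SetState also stops movement for attack, skill and dead states.
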(event `self.ReceiveBeginPlay`
  ;[1 1 1] 최초 시작 상태(PEACE)
  (set `self.CurrentHP` (`self.MaxHP`))
  (`self.SetState` "NewEnumerator0"))

(event `self.PawnSensing.OnSeePawn`
  (params (Pawn :type "Pawn Object Reference"))
  ;[1 1 1] Change State(PEACE->CHASE)
  (if (`|EnumEquality` (`self.CurrentStatePawn`) "NewEnumerator0")
    (set `self.Instigator` Pawn) ; 가해자 변수에 탐지한 pawn 값 저장
    (`self.SetState` "NewEnumerator1")))

(event `self.ReceiveAnyDamage`
  (params (Damage :type "Float (single-precision)") (DamageType :type "DamageType Object Reference") (InstigatedBy :type "Controller Object Reference") (DamageCauser :type "Actor Object Reference"))
  ;[1 1 1] Damage를 받는 이벤트(Another State -> Dead)
  (`SceneComponent.SetVisibility` (`self.BossHealth`) true false)
  (if (`self.bCanBeDamaged`)
    (bind _output_get (set `self.CurrentHP` (- (`self.CurrentHP`) Damage)))
    (if (> _output_get 0.0)
      (`KismetSystemLibrary.PrintString` (`KismetStringLibrary.Conv_DoubleToString` (`self.CurrentHP`)))
      (else
        (`self.SetState` "NewEnumerator3")
        (`KismetSystemLibrary.PrintString` "Dead")))))

(event `self.ReceiveTick`
  (params (DeltaSeconds :type "Float (single-precision)"))
  ;[1 1 1] HP UI
  (bind _asboss_health_bar (cast `/Game/YR/Boss/BossHealthBar` (`WidgetComponent.GetUserWidgetObject` (`self.BossHealth`))))
  (`ProgressBar.SetPercent` (`/Game/YR/Boss/BossHealthBar.Boss_HP` _asboss_health_bar) (/ (`self.CurrentHP`) (`self.MaxHP`))))

(fn `SetState`
  (params (NewState :type "/Game/YR/Boss/BPE_BossState Enum" :default "NewEnumerator0"))
  (locals (ChooseAttackKey :type Name :default "ChooseAttack") (StateKey :type Name :default "State") (NewLocalVar_0 :type "Float (double-precision)" :default 0.0))
  ;[1 1 1] 상태 바꾸는 함수. 상태를 바꾸면 브랙보드의 State도 업데이트함.
  (if (`|EnumInequality` (`self.CurrentStatePawn`) "NewEnumerator3")
    (bind _output_get (set `self.CurrentStatePawn` NewState))
    (`|ExecutionSequence`
      (:`then_0`
        ;;[1 1 1] 블랙보드의 State값에 바뀐 Pawn State를 넣음
        (`BlackboardComponent.SetValueAsEnum` (`AIBlueprintHelperLibrary.GetBlackboard` (`self.GetController`)) (`local.StateKey`) _output_get))
      (:`then_1`
        (switch `/Game/YR/Boss/BPE_BossState` (`self.CurrentStatePawn`)
          (:`NewEnumerator0`
            (set `CharacterMovementComponent.MaxWalkSpeed` 200.0 (`self.CharacterMovement`)))
          (:`NewEnumerator1`
            (set `CharacterMovementComponent.MaxWalkSpeed` (`KismetMathLibrary.RandomFloatInRange` 250.0 500.0) (`self.CharacterMovement`))
            ;[1 1 1] 공격 종류 변수 세팅
            (`BlackboardComponent.SetValueAsInt` (`AIBlueprintHelperLibrary.GetBlackboard` (`self.GetController`)) (`local.ChooseAttackKey`) (`KismetMathLibrary.RandomIntegerInRange` 0 11)))
          (:`NewEnumerator2`
            (set `CharacterMovementComponent.MaxWalkSpeed` 0.0 (`self.CharacterMovement`) :!label _label))
          (:`NewEnumerator3`
            (goto _label))
          (:`NewEnumerator4`
            (goto _label))
          (:`NewEnumerator5`
            (goto _label))
          (:`NewEnumerator6`
            (goto _label)))))))

(fn `UserConstructionScript`)