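; Heal spell Blueprint from the UI Kit showcase, apparently meant to restore health to the casting player's character.
; CastFunction casts the user's controlled pawn to YJPersonCharacter and does nothing further.
; The logic that adds HealAmount capped at MaximumHealth and updates the "health" bar is disconnected, as are leftover nodes that zero health, so casting currently has no effect.
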(event `self.Cast Function`
  (params (User :type "PlayerController Object Reference"))
  (bind _asyjperson_character (cast `/Game/YJ/YJCharacter/YJPersonCharacter` (`Controller.K2_GetPawn` User))))

(fn `UserConstructionScript`
  (`parent.UserConstructionScript`))